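; Arena Blueprint that holds an attack list and the math for resolving attack damage and hit chance in combat.
; BeginPlay fills AttackList with three named attacks: Beam, Kick and Rush.
; DamageCalculator scales raw attack by power, subtracts that total divided by enemy Defense, and clamps the result.
; HitPercentage rolls a weighted random hit from attack accuracy and the speed-to-accuracy ratio, printing debug values on screen.
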(event Custom|Load%20Attack%20Info
  (Variables|Default|SetAttackList (Utilities|Array|MakeArray (Utilities|Struct|MakeAttacks "Beam" 7e+01) (Utilities|Struct|MakeAttacks "Kick" 5e+01 66.0 2e+01 "NewEnumerator0" "NewEnumerator0" "NewEnumerator0") (Utilities|Struct|MakeAttacks "Rush" 6e+01 6e+01 2e+01 "NewEnumerator1" "NewEnumerator0" "NewEnumerator0" 2.0))))

(event EventBeginPlay
  (CallFunction|LoadAttackInfo))

(event EventTick
  (params (DeltaSeconds :type Float%20%28single-precision%29)))

(fn ConstructionScript)

(fn DamageCalculator
  (params (Raw%20Attack :type Float%20%28single-precision%29) (Attack%20Power :type Float%20%28single-precision%29) (Enemy :type Battle%20Cell%20Object%20Reference))
  (bind _returnvalue (* Raw%20Attack Attack%20Power))
  (bind _output_get (Variables|Default|SetAttack%20Total _returnvalue))
  (return (Math|Float|Clamp(Float) (- _output_get (/ _returnvalue (Variables|/Game/PodContent/BluePrints/Cells/BattleCell.BattleCell_C|GetDefense Enemy))) 0.0 1e+03)))

(fn HitPercentage
  (params (AttackerAccuracy :type Float%20%28single-precision%29) (AttackAccuracy :type Float%20%28single-precision%29) (EnemySpeed :type Float%20%28single-precision%29))
  (bind _returnvalue (/ EnemySpeed AttackerAccuracy))
  (bind _returnvalue_2 (/ AttackAccuracy _returnvalue))
  (bind _returnvalue_3 (/ _returnvalue_2 1e+02))
  (Development|PrintString (Utilities|String|ToString(Float) _returnvalue) true true "(R=0.000000,G=1.000000,B=0.000000,A=1.000000)")
  (Development|PrintString (Utilities|String|ToString(Float) _returnvalue_3) true true "(R=1.000000,G=0.000000,B=0.068469,A=1.000000)")
  (return (Math|Random|RandomBoolwithWeight _returnvalue_3)))