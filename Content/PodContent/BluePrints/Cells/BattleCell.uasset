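; BattleCell is a combatant for Arena fights, moving along the X axis opposite an enemy cell.
; On BeginPlay it spawns Legs on Nuke's sockets; Tick sets their animation rate and classifies center distance as close, mid or far range.
; Attacks are sorted by range, while AI selection returns a random attack and movement target.
; MoveToLocation moves both cells under game-mode priority; other events handle heat lockout, cooldown, beam effects and dodging.
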(event Custom|Heat%20Damage
  (bind _self self)
  ;[1 1 1] Heat Damage
  (if (> (Variables|BattleCell_C|GetHeat _self) (Variables|BattleCell_C|GetHeatTolerance _self))
    (Variables|Default|SetcanAttack false)
    (else
      (Variables|Default|SetcanAttack true))))

(event Custom|Move
  (bind _self self)
  (bind _motioncontroller (Variables|BattleCell_C|GetMotionController _self))
  (bind _returnvalue (Transformation|GetWorldLocation _motioncontroller))
  (bind (_x _y _z) (Math|Vector|BreakVector _returnvalue))
  ;[1 1 1] Player Movment
  (if (or (Variables|Default|GetForward) (Variables|Default|GetBackward))
    (if (Variables|Default|GetForward)
      (CallFunction|SetForward)
      (else
        (CallFunction|SetBackwards)))
    (AI|GetAIController _self)
    (bind _output_get (Variables|Default|SetPlayerCellXAxis _x))
    (Transformation|SetWorldLocationAndRotation (Variables|BattleCell_C|GetMotionController _self) (Math|Vector|MakeVector (Math|Float|Clamp(Float) (- _output_get (Variables|Default|GetVelocityIncrese)) (Variables|Default|GetPlayerCellMinX) (Variables|Default|GetPlayerCellMaxX)) _y _z) "0,180.000000, 0" true false)))

(event Custom|SetRange
  (bind _distancetocenter (Variables|Default|GetDistanceToCenter))
  ;[1 1 1] Setting Range
  (if (Math|Float|InRange(Float) _distancetocenter (Variables|Default|GetRange%20Close%20Min) (Variables|Default|GetRange%20Close%20Max))
    (bind _output_get (Variables|Default|SetRangeState "NewEnumerator0"))
    (Development|PrintString (Utilities|String|EnumtoString _output_get) true true "(R=1.000000,G=0.436633,B=0.752964,A=1.000000)" 0.0)
    (elif (Math|Float|InRange(Float) _distancetocenter (Variables|Default|GetRange%20Mid%20Min) (Variables|Default|GetRange%20Mid%20Max) false false)
      (bind _output_get_2 (Variables|Default|SetRangeState "NewEnumerator1"))
      (Development|PrintString (Utilities|String|EnumtoString _output_get_2) true true "(R=0.000000,G=0.660000,B=1.000000,A=1.000000)" 0.0)
      (else
        (bind _output_get_3 (Variables|Default|SetRangeState "NewEnumerator2"))
        (Development|PrintString (Utilities|String|EnumtoString _output_get_3) true true "(R=0.000000,G=0.660000,B=1.000000,A=1.000000)" 0.0)))))

(event Custom|Match%20Distance
  (bind _self self)
  (bind _motioncontroller (Variables|Default|GetMotionController _self))
  (bind _returnvalue (Transformation|GetWorldLocation _motioncontroller))
  (bind (_x _y _z) (Math|Vector|BreakVector _returnvalue))
  ;[1 1 1] Match Distance
  (if (or (Variables|Default|GetForward) (Variables|Default|GetBackward))
    (bind _result (Math|Float|NegateFloat _x)
      (:%20%20
        (Transformation|SetWorldLocationAndRotation (Variables|BattleCell_C|GetMotionController (Variables|Default|GetEnemy)) (Math|Vector|MakeVector _result _y _z) "0, 0, 0" true false)))))

(event Custom|AI%20Move
  ;[1 1 1] AI movment
)

(event Custom|MatchAiLocation
  ;[1 1 1] AI movment
)

(event Custom|Cooldown
  ;[1 1 1] Cool Down
  (Utilities|FlowControl|RetriggerableDelay 0.2 :!label _label)
  (Variables|Default|SetHeat (Math|Float|Clamp(Float) (- (Variables|Default|GetHeat) (Variables|Default|GetCooldownRate)) 0.0 (Variables|Default|GetMax%20Allowed%20Heat)))
  (goto _label))

(event Custom|Dodge
  (bind _self self)
  (bind _returnvalue (Transformation|GetActorLocation _self))
  (bind (_x _y _z) (Math|Vector|BreakVector _returnvalue))
  (Components|MoveComponentTo 0 (Math|Vector|MakeVector _x (+ _y 15.0) _z) "0, 0, 0" false false 0.5 false))

(event Custom|Set%20Attacks
  ;[1 1 1] Setting Attacks Per Cell
  (CallFunction|SortAttacks))

(event Custom|LegSpeed
  (bind _aimovementstate (Variables|Default|GetAiMovementState))
  ;[1 1 1] Leg Movment
  (if (or (or (Utilities|Enum|Equal(Enum) _aimovementstate "NewEnumerator0") (Utilities|Enum|Equal(Enum) _aimovementstate "NewEnumerator1")) (Variables|/Game/PodContent/BluePrints/Arena.Arena_C|GetPlayerMoving (Variables|Default|GetGamemode)))
    (bind _outactors (Actor|GetAllActorsOfClass "/Game/PodContent/BluePrints/Class/Leg.Leg_C"))
    (for _array_element _outactors
      (Components|Timeline|SetPlayRate (Variables|/Game/PodContent/BluePrints/Class/Leg.Leg_C|GetLeg _array_element) 1.5))
    (else
      (bind _outactors_2 (Actor|GetAllActorsOfClass "/Game/PodContent/BluePrints/Class/Leg.Leg_C"))
      (for _array_element_2 _outactors_2
        (Components|Timeline|SetPlayRate (Variables|/Game/PodContent/BluePrints/Class/Leg.Leg_C|GetLeg _array_element_2) 0.0)))))

(event Custom|Beam
  (params (delay :type Float%20%28single-precision%29) (Sound :type Sound%20Wave%20Object%20Reference))
  (bind _returnvalue (Effects|SpawnEmitterAttached "/Game/PodContent/BluePrints/Particles/Test_Beam2.Test_Beam2" (Variables|Default|GetArrow) "None" "0, 0, 0" "0, 0, 0" "SnapToTargetIncludingScale"))
  (Audio|SpawnSoundAttached Sound _returnvalue)
  (Class|ParticleSystemComponent|SetBeamTargetPoint _returnvalue 0 (Transformation|GetWorldLocation (Variables|BattleCell_C|GetNuke (Variables|Default|GetEnemy))))
  (Utilities|FlowControl|Delay delay)
  (Components|DestroyComponent _returnvalue))

(event Custom|Test%20Movment
  (CallFunction|MovetoLocation "NewEnumerator0" self (Variables|Default|GetEnemy)))

(event Custom|Ai%20Attack%20System
  (params (Ai%20Attacker :type Battle%20Cell%20Object%20Reference))
  (CallFunction|AIAttackSelect Ai%20Attacker))

(event Custom|SetBackwards
  ;[1 1 1] Match Distance
  (if (not (< (Variables|Default|GetVelocityIncrese) 0.0))
    (Math|Float|NegateFloat (Variables|Default|GetVelocityIncrese))))

(event Custom|SetForward
  ;[1 1 1] Match Distance
  (if (< (Variables|Default|GetVelocityIncrese) 0.0)
    (Math|Float|NegateFloat (Variables|Default|GetVelocityIncrese))))

(event Custom|StopAiMovment
  (bind _returnvalue (Math|Random|RandomFloatinRange -1e+02 -5e+02))
  (bind _self self)
  (bind _motioncontroller (Variables|Default|GetMotionController _self))
  (bind _returnvalue_2 (Transformation|GetWorldLocation _motioncontroller))
  (bind (_x _y _z) (Math|Vector|BreakVector _returnvalue_2))
  ;[1 1 1] AI movment
  (Components|MoveComponentTo (Variables|Default|GetMotionController) (Math|Vector|MakeVector _returnvalue _y _z) "0, 0, 0" false false (Math|Float|Absolute(Float) (* (.X (Math|Vector|BreakVector (- (Math|Conversions|ToVector(Float) _x) (Math|Conversions|ToVector(Float) _returnvalue)))) 0.01)) false) ; enters at Stop
)

(event Custom|Attach%20Legs
  ;[1 1 1] Attach Components
  (for _array_element (Transformation|GetAllSocketNames (Variables|Default|GetNuke))
    (bind _returnvalue (Game|SpawnActorfromClass "/Game/PodContent/BluePrints/Class/Leg.Leg_C" (Math|Transform|MakeTransform "0, 0, 0" (Variables|Default|GetLegRotation)) "Undefined" 0 0))
    (if (Utilities|String|Contains (Utilities|String|ToString(Name) _array_element) "Leg")
      (Utilities|FlowControl|FlipFlop
        (:A
          (Variables|Default|SetLegRotation "0,180.000000, 0"))
        (:B
          (Variables|Default|SetLegRotation "0,0.000000, 0")))
      (Transformation|AttachComponentToComponent _returnvalue (Variables|Default|GetNuke) _array_element "KeepRelative" "KeepRelative" "KeepRelative" true))))

(event EventBeginPlay
  ;[1 1 1] Begin Play
  (CallFunction|AttachLegs)
  (bind _asarena (Utilities|Casting|CastToArena (Game|GetGameMode)))
  (Variables|Default|SetGamemode _asarena))

(event Collision|EventActorBeginOverlap
  (params (OtherActor :type Actor%20Object%20Reference)))

(event EventTick
  (params (DeltaSeconds :type Float%20%28single-precision%29))
  ;[1 1 1] ON Tick
  (CallFunction|LegSpeed)
  (Variables|Default|SetDistanceToCenter (Transformation|GetHorizontalDistanceTo (Variables|Default|GetCenterPoint)))
  (CallFunction|SetRange))

(event Input|KeyboardEvents|H
  (params (Key :type Key%20Structure :default "AnyKey"))
  ;[1 1 1] Hud Shortcut
  (:Pressed
    (bind _returnvalue (UserInterface|CreateWidget "/Game/PodContent/BluePrints/Hud/Battle_Hud.Battle_Hud_C" (Game|GetPlayerController 0)))
    (bind _output_get (Variables|Default|SetHud _returnvalue))
    (UserInterface|Viewport|AddtoViewport _output_get 0)))

(event Custom|Punch)

(fn ConstructionScript)

(fn SortAttacks
  (bind _myattacks (Variables|Default|GetMyAttacks))
  (for _array_element _myattacks
    (Development|PrintString (.Name (Utilities|Struct|BreakAttacks _array_element)) true true "(R=0.926728,G=0.342099,B=1.000000,A=1.000000)"))
  (for _array_element_2 _myattacks
    (Development|PrintString (.Name (Utilities|Struct|BreakAttacks _array_element_2)))
    (switch Utilities|FlowControl|Switch|SwitchonRange (.Range (Utilities|Struct|BreakAttacks _array_element_2))
      (:NewEnumerator0
        (if (Utilities|Enum|Equal(Enum) (.Range (Utilities|Struct|BreakAttacks _array_element_2)) "NewEnumerator0")
          (Utilities|Array|Add (Variables|Default|GetaCloseRange) _array_element_2)))
      (:NewEnumerator1
        (if (Utilities|Enum|Equal(Enum) (.Range (Utilities|Struct|BreakAttacks _array_element_2)) "NewEnumerator1")
          (Utilities|Array|Add (Variables|Default|GetaMidRange) _array_element_2)))
      (:NewEnumerator2
        (if (Utilities|Enum|Equal(Enum) (.Range (Utilities|Struct|BreakAttacks _array_element_2)) "NewEnumerator2")
          (Development|PrintString (.Name (Utilities|Struct|BreakAttacks _array_element_2)) true true "(R=0.000000,G=0.079200,B=0.120000,A=1.000000)")
          (Utilities|Array|Add (Variables|Default|GetaFarRange) _array_element_2))))))

(fn AttackKick)

(fn AIAttackSelect
  (params (AI :type Battle%20Cell%20Object%20Reference))
  (bind _range_mid_min (Variables|Default|GetRange%20Mid%20Min))
  (bind _range_mid_max (Variables|Default|GetRange%20Mid%20Max))
  (bind _range_far_min (Variables|Default|GetRange%20Far%20Min))
  (bind _range_far_max (Variables|Default|GetRange%20Far%20Max))
  (bind _myattacks (Variables|BattleCell_C|GetMyAttacks AI))
  (bind _returnvalue (Utilities|Array|Length _myattacks))
  (bind _returnvalue_2 (Math|Random|RandomFloatinRange _range_far_min _range_far_max))
  (bind _returnvalue_3 (Math|Random|RandomFloatinRange _range_mid_min _range_mid_max))
  (bind _returnvalue_4 (- _returnvalue 1))
  (bind _returnvalue_5 (Math|Random|RandomIntegerinRange 0 _returnvalue_4))
  (bind _item (Utilities|Array|Get(acopy) _myattacks _returnvalue_5))
  (LocalVariables|SetAi%20Selected%20Attack _item)
  (bind _output_get (LocalVariables|SetSelected%20Attack%20Range (.Range (Utilities|Struct|BreakAttacks _item))))
  (switch Utilities|FlowControl|Switch|SwitchonRange _output_get
    (:NewEnumerator0
      (bind _result (Math|Float|NegateFloat (Math|Random|RandomFloatinRange (Variables|Default|GetRange%20Close%20Min) (Variables|Default|GetRange%20Close%20Max)))
        (:%20%20
          (bind _output_get_2 (LocalVariables|SetVector%20Range (Math|Vector|MakeVector _result 0.0 0.0)))
          (return _output_get_2 (LocalVariables|GetAi%20Selected%20Attack)))))
    (:NewEnumerator1
      (Math|Float|NegateFloat _returnvalue_3
        (:%20%20
          (bind _output_get_3 (LocalVariables|SetVector%20Range (Math|Vector|MakeVector _returnvalue_3 0.0 0.0)))
          (return _output_get_3 (LocalVariables|GetAi%20Selected%20Attack)))))
    (:NewEnumerator2
      (Math|Float|NegateFloat _returnvalue_2
        (:%20%20
          (bind _output_get_4 (LocalVariables|SetVector%20Range (Math|Vector|MakeVector _returnvalue_2 0.0 0.0)))
          (return _output_get_4 (LocalVariables|GetAi%20Selected%20Attack)))))))

(fn MovetoLocation
  (params (Directions :type MovmentDirection%20Enum) (Player :type Battle%20Cell%20Object%20Reference) (Enemy :type Battle%20Cell%20Object%20Reference))
  (bind _gamemode (Variables|Default|GetGamemode))
  (bind _motioncontroller (Variables|BattleCell_C|GetMotionController Enemy))
  (bind _motioncontroller_2 (Variables|BattleCell_C|GetMotionController Player))
  (bind _motioncontroller_3 (Variables|BattleCell_C|GetMotionController Enemy))
  (bind _returnvalue (Transformation|GetWorldLocation _motioncontroller))
  (bind _returnvalue_2 (Transformation|GetWorldLocation _motioncontroller_2))
  (bind (_x _y _z) (Math|Vector|BreakVector _returnvalue))
  (bind (_x_2 _y_2 _z_2) (Math|Vector|BreakVector _returnvalue))
  (bind (_x_3 _y_3 _z_3) (Math|Vector|BreakVector _returnvalue_2))
  (bind (_x_4 _y_4 _z_4) (Math|Vector|BreakVector _returnvalue_2))
  (bind _returnvalue_3 (+ _x_3 -1.0))
  (bind _returnvalue_4 (+ _x_4 1.0))
  (bind _returnvalue_5 (Math|Float|Clamp(Float) _returnvalue_3 1e+02 6e+02))
  (bind _returnvalue_6 (Math|Float|Clamp(Float) _returnvalue_4 1e+02 6e+02))
  (bind _returnvalue_7 (Math|Vector|MakeVector _returnvalue_5 _y_3 _z_3))
  (bind _returnvalue_8 (Math|Vector|MakeVector _returnvalue_6 _y_4 _z_4))
  (bind (_x_5 _y_5 _z_5) (Math|Vector|BreakVector _returnvalue_7))
  (bind (_x_6 _y_6 _z_6) (Math|Vector|BreakVector _returnvalue_8))
  (Development|PrintString (Utilities|String|EnumtoString Directions) true true "(R=0.087808,G=0.110000,B=0.014620,A=1.000000)" 0.0)
  (LocalVariables|SetPlayer_Local Player)
  (LocalVariables|SetEnemy_Local Enemy)
  (switch Utilities|FlowControl|Switch|SwitchonMovmentDirection Directions
    (:NewEnumerator0
      (if (Utilities|Enum|Equal(Enum) (Variables|/Game/PodContent/BluePrints/Arena.Arena_C|GetMovmentPriority (Variables|Default|GetGamemode)) "NewEnumerator1")
        (Transformation|SetRelativeLocation _motioncontroller_2 _returnvalue_7 false false)
        (Transformation|SetRelativeLocation _motioncontroller_3 (Math|Vector|MakeVector (Math|Float|Clamp(Float) (* _x_5 -1.0) -6e+02 -1e+02) _y_5 _z_5) false false)
        (return)))
    (:NewEnumerator1
      (if (Utilities|Enum|Equal(Enum) (Variables|/Game/PodContent/BluePrints/Arena.Arena_C|GetMovmentPriority (Variables|Default|GetGamemode)) "NewEnumerator1")
        (Transformation|SetRelativeLocation _motioncontroller_2 _returnvalue_8 false false)
        (Transformation|SetRelativeLocation _motioncontroller_3 (Math|Vector|MakeVector (Math|Float|Clamp(Float) (* _x_6 -1.0) -6e+02 -1e+02) _y_6 _z_6) false false)
        (return)
        (elif (Utilities|Enum|Equal(Enum) (Variables|/Game/PodContent/BluePrints/Arena.Arena_C|GetMovmentPriority _gamemode) "NewEnumerator0")
          (Variables|/Game/PodContent/BluePrints/Arena.Arena_C|SetMovmentPriority _gamemode "NewEnumerator1"))))
    (:NewEnumerator2
      (if (Utilities|Enum|Equal(Enum) (Variables|/Game/PodContent/BluePrints/Arena.Arena_C|GetMovmentPriority (Variables|Default|GetGamemode)) "NewEnumerator2")
        (Transformation|SetRelativeLocation _motioncontroller (Math|Vector|MakeVector (Math|Float|Clamp(Float) (+ _x 1.0) -6e+02 -1e+02) _y _z) false false)
        (Transformation|SetRelativeLocation (Variables|BattleCell_C|GetMotionController (LocalVariables|GetPlayer_Local)) (Math|Vector|MakeVector (Math|Float|Clamp(Float) (+ (.X (Math|Vector|BreakVector (Transformation|GetWorldLocation (Variables|BattleCell_C|GetMotionController (LocalVariables|GetPlayer_Local))))) 1.0) 1e+02 6e+02) (.Y (Math|Vector|BreakVector (Transformation|GetWorldLocation (Variables|BattleCell_C|GetMotionController (LocalVariables|GetPlayer_Local))))) (.Z (Math|Vector|BreakVector (Transformation|GetWorldLocation (Variables|BattleCell_C|GetMotionController (LocalVariables|GetPlayer_Local)))))) false false)
        (return)
        (elif (Utilities|Enum|Equal(Enum) (Variables|/Game/PodContent/BluePrints/Arena.Arena_C|GetMovmentPriority _gamemode) "NewEnumerator0")
          (Variables|/Game/PodContent/BluePrints/Arena.Arena_C|SetMovmentPriority _gamemode "NewEnumerator1"))))
    (:NewEnumerator3
      (if (Utilities|Enum|Equal(Enum) (Variables|/Game/PodContent/BluePrints/Arena.Arena_C|GetMovmentPriority (Variables|Default|GetGamemode)) "NewEnumerator2")
        (Transformation|SetRelativeLocation _motioncontroller (Math|Vector|MakeVector (Math|Float|Clamp(Float) (+ _x_2 -1.0) -6e+02 -1e+02) _y_2 _z_2) false false)
        (Transformation|SetRelativeLocation (Variables|BattleCell_C|GetMotionController (LocalVariables|GetPlayer_Local)) (Math|Vector|MakeVector (Math|Float|Clamp(Float) (+ (.X (Math|Vector|BreakVector (Transformation|GetWorldLocation (Variables|BattleCell_C|GetMotionController (LocalVariables|GetPlayer_Local))))) -1.0) 1e+02 6e+02) (.Y (Math|Vector|BreakVector (Transformation|GetWorldLocation (Variables|BattleCell_C|GetMotionController (LocalVariables|GetPlayer_Local))))) (.Z (Math|Vector|BreakVector (Transformation|GetWorldLocation (Variables|BattleCell_C|GetMotionController (LocalVariables|GetPlayer_Local)))))) false false)
        (return)))))