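; Cell is an actor, apparently a creature, with a loyalty system that builds trust based on its health.
; A looping one-second delay from BeginPlay runs LoyaltyTick, which raises clamped Trust while health is 20–100% of max and otherwise slowly lowers it.
; Each tick prints Trust and, above a threshold, issues AIMoveTo targeting the player controller rather than its pawn, with no moving Pawn specified.
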(event Custom|Loyalty%20Tick
  (bind _maxhealth (Variables|Default|GetMaxHealth))
  (if (Math|Float|InRange(Float) (Variables|Default|GetCurrentHealth) (* _maxhealth 0.2) _maxhealth)
    (Variables|Default|SetTrust (Math|Float|Clamp(Float) (+ (Variables|Default|GetTrust) 5.0) -1e+02 1e+02))
    (else
      (Variables|Default|SetTrust (Math|Float|Clamp(Float) (- (Variables|Default|GetTrust) 1.0) -1e+02 1e+02))))
  (Development|PrintString (Utilities|String|ToString(Float) (Variables|Default|GetTrust)))
  (if (>= (Variables|Default|GetTrust) 2e+01)
    (AI|AIMoveTo (Variables|Default|GetSkeletalMesh) 0 "0, 0, 0" (Game|GetPlayerController 0) 5.0 true
      (:OnSuccess
        (Development|PrintString "Wait..." true true "(R=1.000000,G=0.226238,B=0.186432,A=1.000000)")))))

(event EventBeginPlay
  (Utilities|FlowControl|RetriggerableDelay 1.0 :!label _label)
  (CallFunction|LoyaltyTick)
  (goto _label))

(event Collision|EventActorBeginOverlap
  (params (OtherActor :type Actor%20Object%20Reference)))

(event EventTick
  (params (DeltaSeconds :type Float%20%28single-precision%29)))

(fn ConstructionScript)

(fn NewFunction0)